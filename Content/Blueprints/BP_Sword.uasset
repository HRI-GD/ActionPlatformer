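; BP_Sword is a Paper2D sword actor that damages BP_Shark or embeds in whatever its box collider hits.
; Overlapping a shark calls its RecieveAttack with fixed damage and destroys the sword.
; A box hit switches the flipbook to a non-looping embedded animation and moves it to the EmbeddedPos offset.
; That hit also sets the box to block the Pawn channel, making the embedded sword solid to pawns.
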(event OnComponentHit(Box)
  (params (HitComponent :type Primitive%20Component%20Object%20Reference) (OtherActor :type Actor%20Object%20Reference) (OtherComp :type Primitive%20Component%20Object%20Reference) (NormalImpulse :type Vector :default "0, 0, 0") (Hit :type Hit%20Result%20Structure%20%28by%20ref%29))
  (Sprite|SetFlipbook (Variables|Default|GetPaperFlipbook) "/Game/PaperAssets/Sword/Captain__Sword_Embedded.Captain__Sword_Embedded")
  (Components|Timeline|SetLooping (Variables|Default|GetPaperFlipbook) false)
  (Transformation|SetRelativeLocation (Variables|Default|GetPaperFlipbook) (Variables|/Script/Engine.SceneComponent|GetRelativeLocation (Variables|Default|GetEmbeddedPos)) false false)
  (Collision|SetCollisionResponsetoChannel (Variables|Default|GetBox) "ECC_Pawn" "ECR_Block"))

(event OnComponentBeginOverlap(Box)
  (params (OverlappedComponent :type Primitive%20Component%20Object%20Reference) (OtherActor :type Actor%20Object%20Reference) (OtherComp :type Primitive%20Component%20Object%20Reference) (OtherBodyIndex :type Integer) (bFromSweep :type Boolean) (SweepResult :type Hit%20Result%20Structure%20%28by%20ref%29))
  (bind _asbp_shark (Utilities|Casting|CastToBP_Shark OtherActor))
  (Default|RecieveAttack _asbp_shark 5e+01)
  (Actor|DestroyActor))

(event EventBeginPlay)

(event Collision|EventActorBeginOverlap
  (params (OtherActor :type Actor%20Object%20Reference)))

(event EventTick
  (params (DeltaSeconds :type Float%20%28single-precision%29)))

(fn ConstructionScript)